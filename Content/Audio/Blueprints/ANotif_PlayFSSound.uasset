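; Anim notify that plays a footstep sound cue at the character's foot during an animation.
; On notify, a left-foot flag picks the left or right foot audio socket on the skeletal mesh and plays the cue at that socket's world location.
; It returns false without playing when no sound cue is assigned.
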(fn `Received_Notify`
  (params (MeshComp :type "SkeletalMeshComponent Object Reference") (Animation :type "AnimSequenceBase Object Reference"))
  (returns (ReturnValue :type Boolean))
  (bind _skeletalmesh (`SkinnedMeshComponent.SkeletalMesh` MeshComp))
  (bind _fssoundcue (`self.FSSoundCue`))
  (`/Engine/EditorBlueprintResources/StandardMacros.IsValid` (`self.FSSoundCue`)
    (:`Is Valid`
      (if (`self.isLeftFoot`)
        (`GameplayStatics.PlaySoundAtLocation` _fssoundcue (`SkeletalMeshSocket.GetSocketLocation` (`SkeletalMesh.FindSocket` _skeletalmesh (`self.LeftFootAudioSocket`)) MeshComp) (struct) 1.0 1.0 0.0 null null null)
        (return true)
        (else
          (`GameplayStatics.PlaySoundAtLocation` _fssoundcue (`SkeletalMeshSocket.GetSocketLocation` (`SkeletalMesh.FindSocket` _skeletalmesh (`self.RightFootAudioSocket`)) MeshComp) (struct) 1.0 1.0 0.0 null null null)
          (return true))))
    (:`Is Not Valid`
      (return false))))